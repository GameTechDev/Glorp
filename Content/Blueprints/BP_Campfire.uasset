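; Campfire actor whose fire effect and sound swell and fade continuously.
; Each Tick advances a fuel level by a signed rate and reverses that rate outside set bounds, so the level ping-pongs without any external input.
; The fuel level drives a particle system float parameter and the audio volume multiplier directly, with a lower bound slightly below zero.
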(event `self.ReceiveTick`
  (params (DeltaSeconds :type "Float (single-precision)"))
  (bind _output_get (set `self.FuelLeft` (+ (`self.FuelLeft`) (* DeltaSeconds (`self.FuelingRate`)))))
  (`ParticleSystemComponent.SetFloatParameter` (`self.ParticleSystemComponent`) "FuelLeft" _output_get)
  (`AudioComponent.SetVolumeMultiplier` (`self.Audio`) _output_get)
  (if (or (<= _output_get -0.2) (>= _output_get 1.0))
    (set `self.FuelingRate` (* (`self.FuelingRate`) -1.0))))

(fn `UserConstructionScript`)