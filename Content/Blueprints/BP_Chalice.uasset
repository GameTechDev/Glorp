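; BP_Chalice is a chalice Blueprint whose particle system is driven by fuel-left and color values.
; SetFuel and SetColor pass those values into the particle system as named parameters.
; After a zero-length delay at BeginPlay it finds and caches the BP_GameUI widget, printing a message if none exists.
; Every tick it reports the active particle count to that UI once found.
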(event `self.ReceiveBeginPlay`
  (`KismetSystemLibrary.Delay` 0.0)
  (bind _foundwidgets (`WidgetBlueprintLibrary.GetAllWidgetsOfClass` "/Game/UI/BP_GameUI.BP_GameUI_C"))
  (if (== (`KismetArrayLibrary.Array_Length` _foundwidgets) 0)
    (`KismetSystemLibrary.PrintString` "GameUI Not Found" true true (struct :`G` 0.66 :`B` 1.0 :`A` 1.0) 5.0)
    (else
      (set `self.GameUI` (`|GetArrayItem` _foundwidgets))
      (set `self.HasGameUI` true))))

(event `self.ReceiveTick`
  (params (DeltaSeconds :type "Float (single-precision)"))
  (`self.ReportParticleAmount`))

(fn `ReportParticleAmount`
  (if (`self.HasGameUI`)
    (`/Game/UI/BP_GameUI.ReportParticles` (`self.GameUI`) (`ParticleSystemComponent.GetNumActiveParticles` (`self.ParticleSystem`)))))

(fn `SetColor`
  (params (Color :type "LinearColor Structure"))
  (`ParticleSystemComponent.SetColorParameter` (`self.ParticleSystem`) "Color" Color))

(fn `SetFuel`
  (params (FuelLeft :type "Float (double-precision)"))
  (`ParticleSystemComponent.SetFloatParameter` (`self.ParticleSystem`) "FuelLeft" FuelLeft))

(fn `UserConstructionScript`)