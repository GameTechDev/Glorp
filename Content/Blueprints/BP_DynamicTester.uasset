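; Interactive particle stress-test actor that spawns and removes BP_GlorpTest systems on key presses, singly or in batches.
; Spawns are offset from the actor by a position counter and width, with hues redistributed as the count changes.
; Keys also adjust the lit percentage and swap all systems between CPU and GPU templates.
; BP_GameUI displays these settings and handles async tick and parallel collision toggles.
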(event `self.ReceiveBeginPlay`
  (`KismetSystemLibrary.Delay` 0.0)
  (bind _foundwidgets (`WidgetBlueprintLibrary.GetAllWidgetsOfClass` "/Game/UI/BP_GameUI.BP_GameUI_C"))
  (bind _output_get (set `self.GameUI` (`|GetArrayItem` _foundwidgets)))
  (set `/Game/UI/BP_GameUI.Particle Prefix` "CPU " _output_get)
  (`self.UpdateLitPercent`))

(event `Key|Add`
  (params (Key :type "Key Structure"))
  (:`Pressed`
    (`self.AddSystem` :!label _label)))

(event `Key|Equals`
  (params (Key :type "Key Structure"))
  (:`Pressed`
    (goto _label)))

(event `Key|Hyphen`
  (params (Key :type "Key Structure"))
  (:`Pressed`
    (`self.RemoveSystem` :!label _label_2)))

(event `Key|Subtract`
  (params (Key :type "Key Structure"))
  (:`Pressed`
    (goto _label_2)))

(event `InputAction|ToggleAsync`
  (params (Key :type "Key Structure"))
  (:`Pressed`
    (`/Game/UI/BP_GameUI.ToggleAysncTick` (`self.GameUI`))))

(event `Key|Multiply`
  (params (Key :type "Key Structure"))
  (:`Pressed`
    (for _ (range 11)
      (`self.AddSystem`))))

(event `InputAction|ToggleParallel`
  (params (Key :type "Key Structure"))
  (:`Pressed`
    (`/Game/UI/BP_GameUI.ToggleParallelCollision` (`self.GameUI`))))

(event `Key|Divide`
  (params (Key :type "Key Structure"))
  (:`Pressed`
    (for _ (range 11)
      (`self.RemoveSystem`))))

(event `Key|Nine`
  (params (Key :type "Key Structure"))
  (:`Pressed`
    (`self.DecrementLit`)))

(event `Key|Zero`
  (params (Key :type "Key Structure"))
  (:`Pressed`
    (`self.IncrementLit`)))

(event `Key|Tab`
  (params (Key :type "Key Structure"))
  (:`Pressed`
    (`self.ToggleGPUSystems`)))

(fn `AddSystem`
  (bind _returnvalue (`|SpawnActorFromClass` "/Game/Blueprints/BP_GlorpTest.BP_GlorpTest_C" (`self.GetNextSpawn`) "Undefined" "OverrideRootScale" null null))
  (if (`self.isGPU`)
    (`ParticleSystemComponent.SetTemplate` (`/Game/Blueprints/BP_GlorpTest.ParticleSystem` _returnvalue) "/Game/Particles/Intel_GlorpSIGGRAPHTest_GPU.Intel_GlorpSIGGRAPHTest_GPU"))
  (`KismetArrayLibrary.Array_Add` (`self.Systems`) _returnvalue)
  (set `self.NextPosition` (+ (`self.NextPosition`) (`self.PositionIncrement`)))
  (`self.RecolorSystems`)
  (`self.UpdateLitPercent`))

(fn `DecrementLit`
  (set `self.LitPercent` (`KismetMathLibrary.FClamp` (- (`self.LitPercent`) (`self.LitIncrement`))))
  (`self.UpdateLitPercent`))

(fn `GetNextSpawn`
  (returns (SpawnHere :type "Transform Structure"))
  (bind _nextposition (`self.NextPosition`))
  (bind _width (`self.Width`))
  (return (`KismetMathLibrary.MakeTransform` (+ (`self.K2_GetActorLocation`) (`KismetMathLibrary.MakeVector` (`KismetMathLibrary.Conv_IntToDouble` (mod _nextposition _width)) (`KismetMathLibrary.Conv_IntToDouble` (* (/ _nextposition _width) (`self.PositionIncrement`))))))))

(fn `IncrementLit`
  (set `self.LitPercent` (`KismetMathLibrary.FClamp` (+ (`self.LitPercent`) (`self.LitIncrement`))))
  (`self.UpdateLitPercent`))

(fn `RecolorSystems`
  (locals (HueIncrement :type "Float (double-precision)") (HueCurrent :type "Float (double-precision)"))
  (set `local.HueIncrement` (/ 360.0 (`KismetMathLibrary.Conv_IntToDouble` (`KismetArrayLibrary.Array_Length` (`self.Systems`)))))
  (for _array_element (`self.Systems`)
    (`/Game/Blueprints/BP_GlorpTest.SetColor` _array_element (`KismetMathLibrary.HSVToRGB` (`local.HueCurrent`) 0.96 0.81))
    (set `local.HueCurrent` (+ (`local.HueCurrent`) (`local.HueIncrement`)))))

(fn `RemoveSystem`
  (locals (ToRemove :type "/Game/Blueprints/BP_GlorpTest Object Reference"))
  (bind _returnvalue (`KismetArrayLibrary.Array_Length` (`self.Systems`)))
  (bind _returnvalue_2 (- _returnvalue 1))
  (if (> _returnvalue 0)
    (set `local.ToRemove` (`|GetArrayItem` (`self.Systems`) _returnvalue_2))
    (`KismetArrayLibrary.Array_Remove` (`self.Systems`) _returnvalue_2)
    (`self.K2_DestroyActor` (`local.ToRemove`))
    (set `self.NextPosition` (- (`self.NextPosition`) (`self.PositionIncrement`)))
    (if (> (`KismetArrayLibrary.Array_Length` (`self.Systems`)) 0)
      (`self.RecolorSystems`))))

(fn `ToggleGPUSystems`
  (if (`self.isGPU`)
    (set `self.isGPU` false)
    (for _array_element (`self.Systems`)
      (`ParticleSystemComponent.SetTemplate` (`/Game/Blueprints/BP_GlorpTest.ParticleSystem` _array_element) "/Game/Particles/Intel_GlorpSIGGRAPHTest.Intel_GlorpSIGGRAPHTest")
      (set `/Game/UI/BP_GameUI.Particle Prefix` "CPU " (`self.GameUI`)))
    (else
      (set `self.isGPU` true)
      (for _array_element_2 (`self.Systems`)
        (`ParticleSystemComponent.SetTemplate` (`/Game/Blueprints/BP_GlorpTest.ParticleSystem` _array_element_2) "/Game/Particles/Intel_GlorpSIGGRAPHTest_GPU.Intel_GlorpSIGGRAPHTest_GPU")
        (set `/Game/UI/BP_GameUI.Particle Prefix` "GPU " (`self.GameUI`))))))

(fn `UpdateLitPercent`
  (bind _litpercent (`self.LitPercent`))
  (`/Game/UI/BP_GameUI.SetPercentLit` (`self.GameUI`) _litpercent)
  (for _array_element (`self.Systems`)
    (`/Game/Blueprints/BP_GlorpTest.SetLitPercent` _array_element _litpercent)))

(fn `UserConstructionScript`)