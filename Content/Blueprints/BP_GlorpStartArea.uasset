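; BP_GlorpStartArea is a per-player start area grouping a start point and two chalices as child actors.
; Its construction script finds the ThirdPersonGlorper with a matching PlayerNum and teleports it to the GlorperPosition component.
; It then tints both chalices with that Glorper's PlayerColor, gives them a zero-based player index, and passes PlayerNum to the start point.
; All of this runs at construction; the event graph is empty.
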(fn `SetupChalice`
  (params (Chalice :type "ChildActorComponent Object Reference") (Color :type "LinearColor Structure") (PlayerIndex :type Integer))
  (bind _asbp_chalice (cast `/Game/Blueprints/BP_Chalice` (`ChildActorComponent.ChildActor` Chalice)))
  (`/Game/Blueprints/BP_Chalice.SetColor` _asbp_chalice Color)
  (set `/Game/Blueprints/BP_Chalice.PlayerIndex` PlayerIndex _asbp_chalice))

(fn `SetupGlorper`
  (bind _outactors (`GameplayStatics.GetAllActorsOfClass` "/Game/Blueprints/ThirdPersonGlorper.ThirdPersonGlorper_C"))
  (for _array_element _outactors
    (if (== (`/Game/Blueprints/ThirdPersonGlorper.PlayerNum` _array_element) (`self.PlayerNum`))
      (bind _output_get (set `self.Glorper` _array_element))
      (`self.K2_SetActorTransform` _output_get (`SceneComponent.K2_GetComponentToWorld` (`self.GlorperPosition`)) false false))))

(fn `UserConstructionScript`
  (bind _returnvalue (- (`self.PlayerNum`) 1))
  (bind _playercolor (`/Game/Blueprints/ThirdPersonGlorper.PlayerColor` (`self.Glorper`)))
  (`self.SetupGlorper`)
  (`self.SetupChalice` (`self.Chalice1`) _playercolor _returnvalue)
  (`self.SetupChalice` (`self.Challice2`) _playercolor _returnvalue)
  (bind _asbp_start_point (cast `/Game/Blueprints/BP_StartPoint` (`ChildActorComponent.ChildActor` (`self.Start Point`))))
  (set `/Game/Blueprints/BP_StartPoint.PlayerNum` (`self.PlayerNum`) _asbp_start_point))