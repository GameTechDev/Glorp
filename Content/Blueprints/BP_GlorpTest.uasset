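; BP_GlorpTest is a test actor for the Glorp particle effect that spins its emitter and reports active particle counts to the game UI.
; BeginPlay picks the lit template if flagged, applies the color, then waits a frame before caching the BP_GameUI widget.
; Tick sets yaw from game time and sends the count once that widget is cached.
; Setter functions change color and split spawning between lit and unlit particles using complementary parameters.
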(event `self.ReceiveBeginPlay`
  (if (`self.IsLit`)
    (`ParticleSystemComponent.SetTemplate` (`self.ParticleSystem`) "/Game/Particles/Intel_GlorpSIGGRAPHLit.Intel_GlorpSIGGRAPHLit"))
  (`ParticleSystemComponent.SetColorParameter` (`self.ParticleSystem`) "Color" (`self.Color`))
  (`KismetSystemLibrary.Delay` 0.0)
  (bind _foundwidgets (`WidgetBlueprintLibrary.GetAllWidgetsOfClass` "/Game/UI/BP_GameUI.BP_GameUI_C" false))
  (set `self.GameUI` (`|GetArrayItem` _foundwidgets))
  (set `self.HasGameUI` true))

(event `self.ReceiveTick`
  (params (DeltaSeconds :type "Float (single-precision)"))
  (if (`self.HasGameUI`)
    (`self.K2_SetActorRotation` (`KismetMathLibrary.MakeRotator` 0.0 0.0 (* (`GameplayStatics.GetTimeSeconds`) (`self.Speed`))))
    (`self.ReportParticleCount`)))

(fn `ReportParticleCount`
  (`/Game/UI/BP_GameUI.ReportParticles` (`self.GameUI`) (`ParticleSystemComponent.GetNumActiveParticles` (`self.ParticleSystem`))))

(fn `SetColor`
  (params (NewColor :type "LinearColor Structure"))
  (bind _output_get (set `self.Color` NewColor))
  (`ParticleSystemComponent.SetColorParameter` (`self.ParticleSystem`) "Color" _output_get))

(fn `SetLitPercent`
  (params (LitPercent :type "Float (double-precision)"))
  (bind _particlesystem (`self.ParticleSystem`))
  (`ParticleSystemComponent.SetFloatParameter` _particlesystem "SpawnLit" LitPercent)
  (`ParticleSystemComponent.SetFloatParameter` _particlesystem "SpawnUnlit" (- 1.0 LitPercent)))

(fn `UserConstructionScript`)