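; Destructible oil drum that releases colored particles when fractured and leaves glorp decals where they collide.
; BeginPlay applies the Color variable to a dynamic drum material and the particle system, and sets ParticleGimbal to absolute rotation.
; Fracturing flags the drum Broken and activates the particles; each collision spawns a BP_GlorpDecal in that color, oriented against the impact velocity.
; Accessor functions expose the broken state and the destructible component.
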(event `self.ReceiveBeginPlay`
  (bind _returnvalue (`KismetMaterialLibrary.CreateDynamicMaterialInstance` "/Game/Materials/M_OilDrum.M_OilDrum"))
  (`MaterialInstanceDynamic.SetVectorParameterValue` _returnvalue "Color" (`self.Color`))
  (`PrimitiveComponent.SetMaterial` (`self.Drum`) 1 _returnvalue)
  (`ParticleSystemComponent.SetColorParameter` (`self.ParticleSystem`) "Color" (`self.Color`))
  (`SceneComponent.SetAbsolute` (`self.ParticleGimbal`) false true false))

(event `self.Drum.OnComponentFracture`
  (params (HitPoint :type "Vector Structure (by ref)") (HitDirection :type "Vector Structure (by ref)"))
  (set `self.Broken` true)
  (`ActorComponent.Activate` (`self.ParticleSystem`) true))

(event `self.ParticleSystem.OnParticleCollide`
  (params (EventName :type Name) (EmitterTime :type "Float (single-precision)") (ParticleTime :type Integer) (Location :type "Vector Structure") (Velocity :type "Vector Structure") (Direction :type "Vector Structure") (Normal :type "Vector Structure") (BoneName :type Name) (PhysMat :type "PhysicalMaterial Object Reference"))
  (`|SpawnActorFromClass` "/Game/Particles/BP_GlorpDecal.BP_GlorpDecal_C" (`KismetMathLibrary.MakeTransform` Location (`KismetMathLibrary.FindLookAtRotation` Velocity (`KismetMathLibrary.MakeVector` 0.0))) "Undefined" "OverrideRootScale" null (`self.Color`) null))

(fn `GetDestructible`
  (returns (NewParam :type "DestructibleComponent Object Reference"))
  (return (`self.Drum`)))

(fn `IsBroken`
  (returns (IsBroken :type Boolean))
  (return (`self.Broken`)))

(fn `UserConstructionScript`)