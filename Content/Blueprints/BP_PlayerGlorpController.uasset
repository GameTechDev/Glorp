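; Player controller for a Glorper pawn that switches it between human and AI control by swapping possession with a spawned AIController.
; A timed intro walks the pawn to its start point, then restores the AI state saved in BP_GlorpGame.
; AI mode periodically reselects targets and glorps at those in range.
; Inputs also rotate controllers across the four players, set colours, and trigger performance toggles and benchmarks.
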(event `self.ReceiveBeginPlay`
  (bind _charactermovement (`Character.CharacterMovement` (`self.GlorpPawn`)))
  ;[1 1 1] Needs to happen after Controllers are made
  (`KismetSystemLibrary.Delay` 0.0)
  (bind _asthird_person_glorper (cast `/Game/Blueprints/ThirdPersonGlorper` (`self.K2_GetPawn`))
    (:`then`
      (bind _output_get (set `self.GlorpPawn` _asthird_person_glorper)))
    (:`CastFailed`
      (bind _glorper (`self.Possess4thGlorper`))
      (bind _output_get_2 (set `self.GlorpPawn` _glorper))))
  (set `Pawn.AIControllerClass` null _output_get)
  (bind _returnvalue (`|SpawnActorFromClass` "/Script/AIModule.AIController" (`KismetMathLibrary.MakeTransform` (0.0 0.0 0.0)) "Undefined" "OverrideRootScale" null null))
  (set `self.AIController` _returnvalue)
  (set `self.PossessedPlayerNum` (`/Game/Blueprints/ThirdPersonGlorper.PlayerNum` (`self.GlorpPawn`)))
  (set `/Game/Blueprints/ThirdPersonGlorper.PlayerController` self (`self.GlorpPawn`))
  ;[0.0319 0.552 0.8148] Start Intro
  (`self.UnPossess`)
  (`self.Possess` (`self.AIController`) (`self.GlorpPawn`))
  (bind _outactors (`GameplayStatics.GetAllActorsOfClass` "/Game/Blueprints/BP_StartPoint.BP_StartPoint_C"))
  (for _array_element _outactors
    (if (== (`/Game/Blueprints/BP_StartPoint.PlayerNum` _array_element) (`/Game/Blueprints/ThirdPersonGlorper.PlayerNum` (`self.GlorpPawn`)))
      (`AIController.MoveToActor` (`self.AIController`) _array_element -1.0 true true true null true)))
  (bind _returnvalue_2 (`KismetSystemLibrary.K2_SetTimerDelegate` (delegate `End Start`) 3.0))
  (set `self.Start Timer` _returnvalue_2)
  (set `self.OGWalkSpeed` (`CharacterMovementComponent.MaxWalkSpeed` _charactermovement))
  (set `CharacterMovementComponent.MaxWalkSpeed` 300.0 _charactermovement))

(event `End Start`
  (set `CharacterMovementComponent.MaxWalkSpeed` (`self.OGWalkSpeed`) (`Character.CharacterMovement` (`self.GlorpPawn`)))
  (`self.StopAI` false)
  (`self.LoadAIState`))

(event `InputAction|ToggleAI`
  (params (Key :type "Key Structure"))
  (:`Pressed`
    (`self.ToggleAI`)))

(event `self.ReceiveTick`
  (params (DeltaSeconds :type "Float (single-precision)"))
  (bind _glorppawn (`self.GlorpPawn`))
  (bind _glorppawn_2 (`self.GlorpPawn`))
  (if (and (`self.isAIControlled`) (`KismetSystemLibrary.IsValid` (`self.GlorpPawn`)))
    (if (or (`KismetSystemLibrary.K2_TimerExistsHandle` (`self.Start Timer`)) (`/Game/Blueprints/ThirdPersonGlorper.IsDead` (`self.GlorpPawn`)))
      (`/Game/Blueprints/ThirdPersonGlorper.StopGlorping` (`self.GlorpPawn`))
      (elif (`KismetSystemLibrary.IsValid` (`/Game/Blueprints/ThirdPersonGlorper.Target` (`self.GlorpPawn`)))
        ;[0.1529 0.521 0.08438] Update Glorping
        (if (<= (`self.GetDistanceTo` _glorppawn (`/Game/Blueprints/ThirdPersonGlorper.Target` _glorppawn)) 270.0)
          (`/Game/Blueprints/ThirdPersonGlorper.EmitGlorp` _glorppawn_2)
          (`self.TurnToTarget`)
          (else
            (`/Game/Blueprints/ThirdPersonGlorper.StopGlorping` _glorppawn_2 :!label _label)))
        (else
          (goto _label))))))

(event `InputAction|SetToRed`
  (params (Key :type "Key Structure"))
  (:`Pressed`
    (`/Game/Blueprints/ThirdPersonGlorper.SetToColorNum` (`self.GlorpPawn`) 0)))

(event `InputAction|SetToBlue`
  (params (Key :type "Key Structure"))
  (:`Pressed`
    (`/Game/Blueprints/ThirdPersonGlorper.SetToColorNum` (`self.GlorpPawn`) 1)))

(event `InputAction|SetToGreen`
  (params (Key :type "Key Structure"))
  (:`Pressed`
    (`/Game/Blueprints/ThirdPersonGlorper.SetToColorNum` (`self.GlorpPawn`) 2)))

(event `InputAction|SetToYellow`
  (params (Key :type "Key Structure"))
  (:`Pressed`
    (`/Game/Blueprints/ThirdPersonGlorper.SetToColorNum` (`self.GlorpPawn`) 3)))

(event `InputAction|ToggleAsync`
  (params (Key :type "Key Structure"))
  (:`Pressed`
    (`/Game/UI/BP_GameUI.ToggleAysncTick` (`/Game/Blueprints/ThirdPersonGlorper.GameUI` (`self.GlorpPawn`)))))

(event `InputAction|ToggleParallel`
  (params (Key :type "Key Structure"))
  (:`Pressed`
    (`/Game/UI/BP_GameUI.ToggleParallelCollision` (`/Game/Blueprints/ThirdPersonGlorper.GameUI` (`self.GlorpPawn`)))))

(event `Key|LeftControl`
  (params (Key :type "Key Structure"))
  (:`Pressed`
    (bind _outactors (`GameplayStatics.GetAllActorsOfClass` "BP_PlayerGlorpController_C"))
    (for _array_element _outactors
      (`self.ToggleAI` _array_element))))

(event `InputAction|RotateControl`
  (params (Key :type "Key Structure"))
  (:`Pressed`
    (`self.RotateAllControls`)))

(event `InputAction|RunBenchmark`
  (params (Key :type "Key Structure"))
  (:`Pressed`
    (bind _outactors (`GameplayStatics.GetAllActorsOfClass` "/Game/Blueprints/BP_Setup.BP_Setup_C"))
    (`/Game/Blueprints/BP_Setup.Run Benchmark` (`|GetArrayItem` _outactors))))

(fn `LoadAIState`
  (bind _asbp_glorp_game (cast `/Game/Blueprints/BP_GlorpGame` (`GameplayStatics.GetGameInstance`)))
  (bind _output (`|GetArrayItem` (`/Game/Blueprints/BP_GlorpGame.PlayerAI` _asbp_glorp_game) (- (`/Game/Blueprints/ThirdPersonGlorper.PlayerNum` (`self.GlorpPawn`)) 1)))
  (if (== _output (`self.isAIControlled`))
    _
    (elif _output
      (`self.StartAI` true)
      (else
        (`self.StopAI` true)))))

(fn `Possess4thGlorper`
  (returns (Glorper :type "/Game/Blueprints/ThirdPersonGlorper Object Reference"))
  (locals (ViewTarget :type "Actor Object Reference"))
  (bind _outactors (`GameplayStatics.GetAllActorsOfClass` "/Game/Blueprints/ThirdPersonGlorper.ThirdPersonGlorper_C"))
  (for _array_element _outactors
    (if (== (`/Game/Blueprints/ThirdPersonGlorper.PlayerNum` _array_element) 4)
      (`self.Possess` _array_element)
      (return _array_element))))

(fn `RotateAllControls`
  (locals (Controllers :type "Array of /Game/Blueprints/BP_PlayerGlorpController Object Reference"))
  (bind _outactors (`GameplayStatics.GetAllActorsOfClass` "/Game/Blueprints/ThirdPersonGlorper.ThirdPersonGlorper_C"))
  (for _array_element _outactors
    (bind _asbp_player_glorp_controller (cast `/Game/Blueprints/BP_PlayerGlorpController` (`/Game/Blueprints/ThirdPersonGlorper.PlayerController` _array_element)))
    (`KismetArrayLibrary.Array_Add` (`local.Controllers`) _asbp_player_glorp_controller))
  (for _array_element_2 (`local.Controllers`)
    (`self.RotateControl` _array_element_2 _outactors)))

(fn `RotateControl`
  (params (AllPlayers :type "Array of /Game/Blueprints/ThirdPersonGlorper Object Reference"))
  (set `self.PossessedPlayerNum` (+ (mod (`self.PossessedPlayerNum`) 4) 1))
  (for _array_element AllPlayers
    (if (== (`/Game/Blueprints/ThirdPersonGlorper.PlayerNum` _array_element) (`self.PossessedPlayerNum`))
      (bind _output_get (set `self.GlorpPawn` _array_element))
      (set `/Game/Blueprints/ThirdPersonGlorper.PlayerController` self _output_get)
      (if (`self.isAIControlled`)
        (`self.Possess` (`self.AIController`) _array_element)
        (else
          (`self.Possess` _array_element)))
      (return))))

(fn `SaveAIState`
  (bind _asbp_glorp_game (cast `/Game/Blueprints/BP_GlorpGame` (`GameplayStatics.GetGameInstance`)))
  (`KismetArrayLibrary.Array_Set` (`/Game/Blueprints/BP_GlorpGame.PlayerAI` _asbp_glorp_game) (- (`/Game/Blueprints/ThirdPersonGlorper.PlayerNum` (`self.GlorpPawn`)) 1) (`self.isAIControlled`)))

(fn `SelectAITarget`
  (`/Game/Blueprints/ThirdPersonGlorper.SelectAITarget` (`self.GlorpPawn`) (`self.AIController`)))

(fn `StartAI`
  (params (ShouldSaveChange :type Boolean :default true))
  (`self.SelectAITarget`)
  (`KismetSystemLibrary.K2_SetTimer` null "SelectAITarget" (`KismetMathLibrary.RandomFloatInRange` 0.4 0.6) true)
  (`self.UnPossess`)
  (`self.Possess` (`self.AIController`) (`self.GlorpPawn`))
  (set `self.isAIControlled` true)
  (if ShouldSaveChange
    (`self.SaveAIState`)))

(fn `StopAI`
  (params (ShouldSaveChange :type Boolean :default true))
  (locals (OGViewTarget :type "Actor Object Reference"))
  (set `local.OGViewTarget` (`self.GetViewTarget`))
  (`self.StopMovement`)
  (`/Game/Blueprints/ThirdPersonGlorper.StopGlorping` (`self.GlorpPawn`))
  (`KismetSystemLibrary.K2_ClearTimer` null "SelectAITarget")
  (`self.UnPossess` (`self.AIController`))
  (`self.Possess` (`self.GlorpPawn`))
  (`self.SetViewTargetWithBlend` (`local.OGViewTarget`))
  (set `self.isAIControlled` false)
  (if ShouldSaveChange
    (`self.SaveAIState`)))

(fn `ToggleAI`
  ;[1 1 1] Only switch if not in intro
  (if (not (`KismetSystemLibrary.K2_TimerExistsHandle` (`self.Start Timer`)))
    (if (`self.isAIControlled`)
      (`self.StopAI` true)
      (else
        (`self.StartAI` true)))))

(fn `TurnToTarget`
  (bind _glorppawn (`self.GlorpPawn`))
  (bind _yaw (.yaw (`KismetMathLibrary.FindLookAtRotation` (`self.K2_GetActorLocation` (`/Game/Blueprints/ThirdPersonGlorper.Target` _glorppawn)) (`self.K2_GetActorLocation` _glorppawn))))
  (`self.K2_SetActorRotation` (`self.GlorpPawn`) (`KismetMathLibrary.MakeRotator` 0.0 0.0 (+ (`KismetMathLibrary.Lerp` _yaw _yaw (`KismetMathLibrary.FMin` (* (`GameplayStatics.GetWorldDeltaSeconds`) 1.0) 1.0)) 180.0)) false))

(fn `UserConstructionScript`)