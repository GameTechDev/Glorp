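; BP_Setup runs one-time startup configuration for the game, guarded by a flag on the BP_GlorpGame game instance.
; On first BeginPlay it raises the FPS cap and turns on unit and FPS stat displays through console commands.
; It then runs a hardware benchmark, applies the resulting user settings, and prints the visual effect quality on screen.
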(event `self.ReceiveBeginPlay`
  (bind _asbp_glorp_game (cast `/Game/Blueprints/BP_GlorpGame` (`GameplayStatics.GetGameInstance`)))
  (if (not (`/Game/Blueprints/BP_GlorpGame.AreStatsActive` _asbp_glorp_game))
    (set `/Game/Blueprints/BP_GlorpGame.AreStatsActive` true _asbp_glorp_game)
    ;[0.1529 0.521 0.08438] Starting commands
    (`KismetSystemLibrary.ExecuteConsoleCommand` "t.MaxFPS 500" null)
    (`KismetSystemLibrary.ExecuteConsoleCommand` "stat unit" null)
    (`KismetSystemLibrary.ExecuteConsoleCommand` "stat fps" null)
    (`self.Run Benchmark`)))

(fn `Run Benchmark`
  (bind _returnvalue (`GameUserSettings.GetGameUserSettings`))
  (`GameUserSettings.RunHardwareBenchmark` _returnvalue 10 1.0 1.0)
  (`GameUserSettings.ApplyHardwareBenchmarkResults` _returnvalue)
  (`KismetSystemLibrary.PrintString` (`KismetTextLibrary.Conv_TextToString` (`|FormatText` "Effect quality set to: {Quality}" (`KismetTextLibrary.Conv_StringToText` (`self.GetQualityName` (`GameUserSettings.GetVisualEffectQuality` _returnvalue))))) true true (struct :`G` 0.66 :`B` 1.0 :`A` 1.0) 5.0))

(fn `UserConstructionScript`)