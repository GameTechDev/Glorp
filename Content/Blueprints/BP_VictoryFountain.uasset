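; BP_VictoryFountain is a particle fountain that shows the color of the last winning player.
; On BeginPlay it activates the effect and tints it from PlayerColors using LastWinColorNum in BP_GlorpGame, only when that index is non-negative.
; After a zero-length delay it caches the BP_GameUI widget, then reports the active particle count to that UI every Tick.
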(event `self.ReceiveBeginPlay`
  (`self.InitFountainColor`)
  (`KismetSystemLibrary.Delay` 0.0)
  (bind _foundwidgets (`WidgetBlueprintLibrary.GetAllWidgetsOfClass` "/Game/UI/BP_GameUI.BP_GameUI_C"))
  (set `self.GameUI` (`|GetArrayItem` _foundwidgets))
  (set `self.hasGameUI` true)
  (bind _asbp_glorp_game (cast `/Game/Blueprints/BP_GlorpGame` (`GameplayStatics.GetGameInstance`)))
  (set `self.Game Instance` _asbp_glorp_game))

(event `self.ReceiveTick`
  (params (DeltaSeconds :type "Float (single-precision)"))
  (if (`self.hasGameUI`)
    (`/Game/UI/BP_GameUI.ReportParticles` (`self.GameUI`) (`ParticleSystemComponent.GetNumActiveParticles` (`self.Fountatin`)))))

(fn `InitFountainColor`
  (bind _asbp_glorp_game (cast `/Game/Blueprints/BP_GlorpGame` (`GameplayStatics.GetGameInstance`)))
  (bind _lastwincolornum (`/Game/Blueprints/BP_GlorpGame.LastWinColorNum` _asbp_glorp_game))
  (if (>= _lastwincolornum 0)
    (`ActorComponent.Activate` (`self.Fountatin`) false)
    (`ParticleSystemComponent.SetColorParameter` (`self.Fountatin`) "Color" (`|GetArrayItem` (`self.PlayerColors`) _lastwincolornum))))

(fn `UserConstructionScript`)