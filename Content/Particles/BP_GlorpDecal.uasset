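; BP_GlorpDecal is a short-lived, colored splat decal with randomized roll, scale and texture.
; On BeginPlay it destroys itself if its collider overlaps more than MaxOverlaps other glorp decals, limiting stacking.
; Otherwise it applies a dynamic material for texture and color, then sets timers for fade and death.
; During the fade, Tick lowers material opacity linearly until the actor is destroyed at Lifetime.
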(event `self.ReceiveBeginPlay`
  (if (`self.ShouldExist`)
    (`KismetSystemLibrary.K2_SetTimerDelegate` (delegate `Fade`) (- (`self.Lifetime`) (`self.FadeOutTime`)))
    (`KismetSystemLibrary.K2_SetTimerDelegate` (delegate `Death`) (`self.Lifetime`))
    (set `self.StartTime` (`GameplayStatics.GetTimeSeconds`))
    ;[1 1 1] Set up dynamic materials for fade out later
    (bind _returnvalue (`KismetMaterialLibrary.CreateDynamicMaterialInstance` "/Game/Particles/M_GlorpDecal.M_GlorpDecal"))
    (bind _output_get (set `self.GlorpMaterial` _returnvalue))
    (`DecalComponent.SetDecalMaterial` (`self.Decal`) _output_get)
    (`MaterialInstanceDynamic.SetTextureParameterValue` (`self.GlorpMaterial`) "Texture" (`|GetArrayItem` (`self.SplatTextures`) (`KismetMathLibrary.RandomInteger` (- (`KismetArrayLibrary.Array_Length` (`self.SplatTextures`)) 1))))
    (`MaterialInstanceDynamic.SetVectorParameterValue` (`self.GlorpMaterial`) "Color" (`self.Color`))
    (else
      (`self.K2_DestroyActor`))))

(event `Fade`
  (set `self.Fading` true))

(event `Death`
  (`self.K2_DestroyActor`))

(event `self.ReceiveTick`
  (params (DeltaSeconds :type "Float (single-precision)"))
  ;[1 1 1] Handle Fading
  (if (`self.Fading`)
    (`MaterialInstanceDynamic.SetScalarParameterValue` (`self.GlorpMaterial`) "Opacity" (/ (- (+ (`self.StartTime`) (`self.Lifetime`)) (`GameplayStatics.GetTimeSeconds`)) (`self.FadeOutTime`)))))

(fn `ShouldExist`
  (returns (ShouldExist :type Boolean))
  (return (<= (`KismetArrayLibrary.Array_Length` (`PrimitiveComponent.GetOverlappingActors` (`self.Collider`) "BP_GlorpDecal_C")) (`self.MaxOverlaps`))))

(fn `UserConstructionScript`
  (locals (RandScale :type "Float (double-precision)" :default 0.0))
  (bind _returnvalue (`KismetMathLibrary.RandomFloatInRange` 0.8 1.2))
  (`self.K2_AddActorLocalRotation` (`KismetMathLibrary.MakeRotator` (`KismetMathLibrary.RandomFloatInRange` 0.0 360.0)))
  (set `local.RandScale` _returnvalue)
  (`self.SetActorScale3D` (`KismetMathLibrary.Conv_DoubleToVector` _returnvalue))
  (`SceneComponent.SetWorldScale3D` (`self.Collider`) (1.25 1.25 1.25)))