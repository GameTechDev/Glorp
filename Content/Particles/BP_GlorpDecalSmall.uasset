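; BP_GlorpDecalSmall is a short-lived glorp splat decal that fades out and destroys itself.
; The construction script pitches it 90 degrees and randomizes roll and scale.
; On BeginPlay, ShouldExist gates spawning (always true here), then timers are set and a dynamic material gets a random splat texture and color.
; Once the fade timer fires, Tick lowers material opacity over FadeOutTime until the death timer destroys the actor.
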(event `self.ReceiveBeginPlay`
  (if (`self.ShouldExist`)
    (`KismetSystemLibrary.K2_SetTimerDelegate` (delegate `Fade`) (- (`self.Lifetime`) (`self.FadeOutTime`)))
    (`KismetSystemLibrary.K2_SetTimerDelegate` (delegate `Death`) (`self.Lifetime`))
    (set `self.StartTime` (`GameplayStatics.GetTimeSeconds`))
    ;[1 1 1] Set up dynamic materials for fade out later
    (bind _returnvalue (`KismetMaterialLibrary.CreateDynamicMaterialInstance` "/Game/Particles/M_GlorpDecal.M_GlorpDecal"))
    (bind _output_get (set `self.GlorpMaterial` _returnvalue))
    (`DecalComponent.SetDecalMaterial` (`self.Decal`) _output_get)
    (`MaterialInstanceDynamic.SetTextureParameterValue` (`self.GlorpMaterial`) "Texture" (`|GetArrayItem` (`self.SplatTextures`) (`KismetMathLibrary.RandomInteger` (- (`KismetArrayLibrary.Array_Length` (`self.SplatTextures`)) 1))))
    (`MaterialInstanceDynamic.SetVectorParameterValue` (`self.GlorpMaterial`) "Color" (`self.Color`))
    (else
      (`self.K2_DestroyActor`))))

(event `Fade`
  (set `self.Fading` true))

(event `Death`
  (`self.K2_DestroyActor`))

(event `self.ReceiveTick`
  (params (DeltaSeconds :type "Float (single-precision)"))
  ;[1 1 1] Handle Fading
  (if (`self.Fading`)
    (`MaterialInstanceDynamic.SetScalarParameterValue` (`self.GlorpMaterial`) "Opacity" (/ (- (+ (`self.StartTime`) (`self.Lifetime`)) (`GameplayStatics.GetTimeSeconds`)) (`self.FadeOutTime`)))))

(fn `ShouldExist`
  (returns (ShouldExist :type Boolean))
  (return true))

(fn `UserConstructionScript`
  (`self.K2_SetActorRotation` (`KismetMathLibrary.MakeRotator` (`KismetMathLibrary.RandomFloatInRange` 0.0 360.0) 90.0))
  (`self.SetActorScale3D` (`KismetMathLibrary.Conv_DoubleToVector` (`KismetMathLibrary.RandomFloatInRange` 0.8 1.2))))